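; Farm plot actor that can be watered, seeded and harvested, with a state running from Empty through Growing to Harvestable.
; Seed starts growth, and Tick raises the Wheat component until it passes a world-height threshold, then marks it Harvestable.
; Water only tints the soil material to WetColor.
; Harvest restores the start color, empties the state and moves Wheat to a fixed world position, not one relative to the plot.
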(event EventBeginPlay
  (Rendering|SetVisibility (Variables|Default|GetGrass_1) false false)
  (Rendering|Material|SetVectorParameterValueonMaterials (Variables|Default|GetFarm_Farm) "Color" (Math|Conversions|ToVector(LinearColor) (Math|Conversions|ToLinearColor(Color) (Variables|Default|GetStartColor)))))

(event Collision|EventActorBeginOverlap
  (params (OtherActor :type Actor%20Object%20Reference)))

(event EventTick
  (params (DeltaSeconds :type Float%20%28single-precision%29))
  (bind _wheat (Variables|Default|GetWheat))
  (switch Utilities|FlowControl|Switch|SwitchonLandState (Variables|Default|GetState)
    (:NewEnumerator1
      ;[1 1 1] Growth
      (if (<= (.z (Transformation|GetWorldLocation _wheat)) 6e+01)
        (Transformation|AddWorldOffset _wheat (Math|Vector|MakeVector 0.0 0.0 (* DeltaSeconds 1e+02)) false false)
        (else
          (Variables|Default|SetState "NewEnumerator2")
          (Development|PrintString "GROWN!"))))))

(fn ConstructionScript)

(fn Water
  (Development|PrintString "WATER CHANGE COLOR")
  (Rendering|Material|SetVectorParameterValueonMaterials (Variables|Default|GetFarm_Farm) "Color" (Math|Conversions|ToVector(LinearColor) (Math|Conversions|ToLinearColor(Color) (Variables|Default|GetWetColor)))))

(fn Seed
  (Variables|Default|SetState "NewEnumerator1"))

(fn Harvest
  (Transformation|SetWorldLocation (Variables|Default|GetWheat) "0, 0,-50.000000" false false)
  (Variables|Default|SetState "NewEnumerator0")
  (Rendering|Material|SetVectorParameterValueonMaterials (Variables|Default|GetFarm_Farm) "Color" (Math|Conversions|ToVector(LinearColor) (Math|Conversions|ToLinearColor(Color) (Variables|Default|GetStartColor)))))